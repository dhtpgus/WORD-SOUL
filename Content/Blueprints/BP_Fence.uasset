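; BP_Fence is a procedural fence actor that lays out a straight row of static mesh segments toward its FenceEnd point.
; The construction script flattens FenceEnd to zero Z, derives length and direction, then adds aligned mesh components at a fixed spacing for as many as fit.
; Each segment gets a slight random height scale, while the yaw jitter and local offset are zeroed.
; The event graph has no runtime logic.
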(event EventBeginPlay)

(event Collision|EventActorBeginOverlap
  (params (OtherActor :type Actor%20Object%20Reference)))

(event EventTick
  (params (DeltaSeconds :type Float%20%28single-precision%29)))

(fn ConstructionScript
  (Variables|Default|SetFenceEnd (Math|Vector|MakeVector (.x (Variables|Default|GetFenceEnd)) (.y (Variables|Default|GetFenceEnd)) 0.0))
  (Variables|Default|SetLength (Math|Vector|VectorLength (Variables|Default|GetFenceEnd)))
  (Variables|Default|SetFenceDirection (Math|Vector|GetUnitDirection(Vector) "0, 0, 0" (Variables|Default|GetFenceEnd)))
  (Variables|Default|SetFenceRotation (Math|Conversions|RotationFromXVector (Math|Vector|GetUnitDirection(Vector) "0, 0, 0" (Variables|Default|GetFenceEnd))))
  (for _index (range 0 (Math|Float|Truncate (- (/ (Variables|Default|GetLength) 1.27e+03) 1.0)))
    (bind _returnvalue (AddComponent|AddStaticMeshComponent false (Math|Transform|MakeTransform (* _index 1270 (Variables|Default|GetFenceDirection)) (Math|Rotator|CombineRotators (Variables|Default|GetFenceRotation) (Math|Rotator|MakeRotator 0.0 0.0 (Math|Random|RandomFloatinRange 0.0 0.0))) (Math|Vector|MakeVector 1.0 1.0 (Math|Random|RandomFloatinRange 0.9 1.0)))))
    (Transformation|AddLocalOffset _returnvalue "0, 0, 0" false false)))