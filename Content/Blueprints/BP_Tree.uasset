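; BP_Tree is an actor that procedurally scatters static mesh trees within a box volume.
; Its construction script loops by TreeCount, adding a static mesh component at a random X/Y point inside the Box bounds, with Z left at zero.
; Each mesh gets random yaw and uniform scale from unseeded random nodes, so the layout changes whenever construction reruns.
; The event graph holds only unused default events.
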(event EventBeginPlay)

(event Collision|EventActorBeginOverlap
  (params (OtherActor :type Actor%20Object%20Reference)))

(event EventTick
  (params (DeltaSeconds :type Float%20%28single-precision%29)))

(fn ConstructionScript
  (bind _box (Variables|Default|GetBox))
  (bind _relativelocation (Variables|/Script/Engine.SceneComponent|GetRelativeLocation _box))
  (bind _boxextent (Variables|/Script/Engine.BoxComponent|GetBoxExtent _box))
  (bind _returnvalue (Math|Random|RandomPointinBoundingBox _relativelocation _boxextent))
  (bind (_x _y) (Math|Vector|BreakVector _returnvalue))
  (for _index (range 0 (Variables|Default|GetTreeCount))
    (AddComponent|AddStaticMeshComponent false (Math|Transform|MakeTransform (Math|Vector|MakeVector _x _y 0.0) (Math|Rotator|MakeRotator 0.0 0.0 (Math|Random|RandomFloatinRange 0.0 3.6e+02)) (Math|Conversions|ToVector(Float) (Math|Random|RandomFloatinRange 0.4 1.0))))))